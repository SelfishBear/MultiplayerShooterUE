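; Multiplayer shooter player controller that toggles the game info panel on the local player's HUD and cycles graphics quality.
; On BeginPlay it binds to BP_MS_BaseHUD's widget-initialized event to cache the WBP_BasePlayerHUD reference.
; ShowGameInfo re-fetches the widget from the HUD if the cached reference is invalid, while HideGameInfo uses it unchecked.
; ChangeGraphics increments an index, wraps it across five overall scalability levels and applies the setting.
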(event `self.ReceiveBeginPlay`
  (`self.InitMSHUD`))

(event `self.ShowGameInfo`
  (if (`self.IsLocalController`)
    (`/Engine/EditorBlueprintResources/StandardMacros.IsValid` (`self.Base HUD Widget`)
      (:`Is Valid`
        (`Widget.SetVisibility` (`/Game/MultiplayerShooter/Blueprint/UI/WBP_BasePlayerHUD.GetGameInfo` (`self.Base HUD Widget`)) "Visible"))
      (:`Is Not Valid`
        (`self.RetryGetWidget`)
        (`Widget.SetVisibility` (`/Game/MultiplayerShooter/Blueprint/UI/WBP_BasePlayerHUD.GetGameInfo` (`self.Base HUD Widget`)) "Visible")))))

(event `self.HideGameInfo`
  (if (`self.IsLocalController`)
    (`Widget.SetVisibility` (`/Game/MultiplayerShooter/Blueprint/UI/WBP_BasePlayerHUD.GetGameInfo` (`self.Base HUD Widget`)) "Hidden")))

(event `self.ChangeGraphics`
  (bind _result (`/Engine/EditorBlueprintResources/StandardMacros.IncrementInt` (`self.GraphicsIndex`))
    (:`  `
      (bind _returnvalue (`GameUserSettings.GetGameUserSettings`))
      (`GameUserSettings.SetOverallScalabilityLevel` _returnvalue (mod _result 5))
      (`GameUserSettings.ApplySettings` _returnvalue true))))

(fn `InitMSHUD`
  (if (`self.IsLocalController`)
    (bind _asbp_ms_base_hud (cast `/Game/MultiplayerShooter/Blueprint/Core/BP_MS_BaseHUD` (`self.GetHUD`)))
    (add `MS_BaseHUD.OnBaseHUDWidgetInitialized` _asbp_ms_base_hud (`|CreateDelegate` :!event `OnBaseHUDWidgetInit`))))

(fn `OnBaseHUDWidgetInit`
  (params (BaseHUDWidget :type "UserWidget Object Reference"))
  (`/Engine/EditorBlueprintResources/StandardMacros.IsValid` BaseHUDWidget
    (:`Is Valid`
      (bind _aswbp_base_player_hud (cast `/Game/MultiplayerShooter/Blueprint/UI/WBP_BasePlayerHUD` BaseHUDWidget))
      (`/Engine/EditorBlueprintResources/StandardMacros.IsValid` _aswbp_base_player_hud
        (:`Is Valid`
          (set `self.Base HUD Widget` _aswbp_base_player_hud))))))

(fn `RetryGetWidget`
  (bind _asbp_ms_base_hud (cast `/Game/MultiplayerShooter/Blueprint/Core/BP_MS_BaseHUD` (`self.GetHUD`)))
  (`/Engine/EditorBlueprintResources/StandardMacros.IsValid` _asbp_ms_base_hud
    (:`Is Valid`
      (bind _aswbp_base_player_hud (cast `/Game/MultiplayerShooter/Blueprint/UI/WBP_BasePlayerHUD` (`MS_BaseHUD.PlayerBaseHUDWidget` _asbp_ms_base_hud)))
      (`/Engine/EditorBlueprintResources/StandardMacros.IsValid` _aswbp_base_player_hud
        (:`Is Valid`
          (set `self.Base HUD Widget` _aswbp_base_player_hud))))))

(fn `UserConstructionScript`)