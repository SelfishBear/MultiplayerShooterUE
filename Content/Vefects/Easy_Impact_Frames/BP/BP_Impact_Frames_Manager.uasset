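; BP_Impact_Frames_Manager is an actor set up as a keyboard trigger for impact frame effects from the Vefects Easy Impact Frames content.
; On BeginPlay it enables input for player controller 0, and pressing 1 calls the Impact event, which is empty here.
; Disconnected nodes that never run would play a world camera shake and spawn the impact frame and extra VFX systems at the actor's location.
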(event `self.ReceiveBeginPlay`
  (`self.EnableInput` (`GameplayStatics.GetPlayerController` 0)))

(event `Key|One`
  (params (Key :type "Key Structure"))
  (:`Pressed`
    (`self.Impact`)))

(event `Impact`)

(fn `UserConstructionScript`)